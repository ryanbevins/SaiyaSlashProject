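; Player character Blueprint for Farak, adding jump, sprint, targeting input and camera zoom.
; Jumps from the ground play a start montage, launch after a short delay, and stop the montage on landing.
; A timeline eases camera boom length for zoom, and debug mode adds a debug widget.
; The gamepad right shoulder calls TryBeginTargetting; OnTarget and Tick's target check are stubs, and the sphere-trace target searches are disconnected.
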(event `self.ReceiveBeginPlay`
  (if (`self.DebugMode?`)
    (bind _returnvalue (`|CreateWidget` "/Game/Blueprints/Game/Debug/UMG_Debug.UMG_Debug_C" (`self.GetLocalViewingPlayerController`)))
    (bind _output_get (set `self.DebugWidget` _returnvalue))
    (`UserWidget.AddToViewport` _output_get 0)))

(event `self.OnStartJump`
  (bind _returnvalue (`SkeletalMeshComponent.GetAnimInstance` (`self.Mesh`)))
  (if (`NavMovementComponent.IsMovingOnGround` (`self.CharacterMovement`))
    (if (not (`AnimInstance.Montage_IsPlaying` _returnvalue "/Game/Characters/NovaStrike/Farak/Animations/Movement/Player/JumpStart_UE5_Montage.JumpStart_UE5_Montage"))
      (`AnimInstance.Montage_Play` _returnvalue "/Game/Characters/NovaStrike/Farak/Animations/Movement/Player/JumpStart_UE5_Montage.JumpStart_UE5_Montage" 1.0 "MontageLength" 0.0 true)
      (`KismetSystemLibrary.Delay` 0.15)
      (`self.Jump`))))

(event `self.OnJumped`
  (`parent.OnJumped`))

(event `self.ReceiveTick`
  (params (DeltaSeconds :type "Float (single-precision)"))
  (`/Engine/EditorBlueprintResources/StandardMacros.IsValid` (`self.TargetEnemy`)))

(event `self.OnLanded`
  (params (Hit :type "HitResult Structure (by ref)"))
  (`parent.OnLanded` Hit)
  (`AnimInstance.Montage_Stop` (`SkeletalMeshComponent.GetAnimInstance` (`self.Mesh`)) 0.25 "/Game/Characters/NovaStrike/Farak/Animations/Movement/Player/JumpStart_UE5_Montage.JumpStart_UE5_Montage"))

(event `InputAction|Sprint`
  (params (Key :type "Key Structure"))
  (:`Pressed`
    (`self.Sprint`))
  (:`Released`
    (`self.StopSprint`)))

(event `Key|Gamepad_RightShoulder`
  (params (Key :type "Key Structure"))
  (:`Pressed`
    (`self.TryBeginTargetting`)))

(event `self.OnTarget`
  (`KismetSystemLibrary.Delay` 0.0))

(event `self.ZoomCamera`
  (params (DesiredArmLength :type "Float (single-precision)"))
  (set `self.CameraArmLengthBeforeZoom` (`SpringArmComponent.TargetArmLength` (`self.CameraBoom`)))
  (`TimelineComponent.SetPlayRate` (`self.ZoomCameraTimeline`) (`self.CameraZoomSpeed`))
  (bind (_direction _alpha) (`Timeline|ZoomCameraTimeline` :!via `PlayFromStart`)
    (:`Update`
      (set `SpringArmComponent.TargetArmLength` (`|EaseFunction` "EaseInOut" _alpha (`self.CameraArmLengthBeforeZoom`) DesiredArmLength) (`self.CameraBoom`)))))

(fn `UserConstructionScript`)